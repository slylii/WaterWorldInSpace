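; BP_AISub is a trigger actor that shows a subtitle, apparently an AI line, when the first-person player character overlaps its Box.
; On overlap it passes SubName to BP_FirstPersonCharacter, turns the subtitle on, then hides it after a ShowLenght delay.
; A WasActive flag makes it fire only once until the Reboot event clears it.
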(event `self.Box.OnComponentBeginOverlap`
  (params (OverlappedComponent :type "PrimitiveComponent Object Reference") (OtherActor :type "Actor Object Reference") (OtherComp :type "PrimitiveComponent Object Reference") (OtherBodyIndex :type Integer) (bFromSweep :type Boolean) (SweepResult :type "HitResult Structure (by ref)"))
  (if (not (`self.bWasActive`))
    (bind _asbp_first_person_character (cast `/Game/FirstPerson/Blueprints/BP_FirstPersonCharacter` OtherActor))
    (`/Game/FirstPerson/Blueprints/BP_FirstPersonCharacter.UpdateSubtitle` _asbp_first_person_character (`self.SubName`))
    (set `self.bWasActive` true)
    (`/Game/FirstPerson/Blueprints/BP_FirstPersonCharacter.ChangeSubtitleState` _asbp_first_person_character true)
    (`KismetSystemLibrary.Delay` (`self.ShowLenght`))
    (`/Game/FirstPerson/Blueprints/BP_FirstPersonCharacter.ChangeSubtitleState` _asbp_first_person_character false)))

(event `/Game/Interfaces/BPI_Reboot.Reboot`
  (set `self.bWasActive` false))

(fn `UserConstructionScript`)