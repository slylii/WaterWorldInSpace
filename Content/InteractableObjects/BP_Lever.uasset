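; BP_Lever is an interactable lever that works only once its repair flag is set, and only one time.
; On interact it plays a sound, marks itself active and starts a timeline that incrementally rolls Cube1 by a scaled Speed track.
; Each timeline update also sends RebootMessage to RebootActors, so the message repeats throughout the animation rather than firing once.
; The Repair event sets the flag that unlocks the lever.
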(event `/Game/Interfaces/BPI_InteractObject.OnInteract`
  (if (`self.bIsRepair`)
    (if (not (`self.bIsActive`))
      (`GameplayStatics.PlaySoundAtLocation` "/Game/Sounds/SW_OpenDoor.SW_OpenDoor" (`self.K2_GetActorLocation`) (struct) 1.0 1.0 0.0 null null null null)
      (set `self.bIsActive` true)
      (bind (_direction _speed) (`Timeline|LeverTL`)
        (:`Update`
          (`SceneComponent.K2_AddLocalRotation` (`self.Cube1`) (`KismetMathLibrary.MakeRotator` (* _speed 0.6)) false false)
          (message `/Game/Interfaces/BPI_Reboot.Reboot` (`self.RebootActors`)))))))

(event `/Game/Interfaces/BPI_Repair.Repair`
  (params (bIsRepair :type Boolean))
  (set `self.bIsRepair` bIsRepair))

(fn `UserConstructionScript`)