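; BP_OxygenHub is an interactable station that refills the first-person player's oxygen.
; Interacting while IsActive is false replenishes oxygen, updates its UI, plays a pickup sound and sets IsActive, blocking further use.
; That interaction also sends reboot messages to two linked doors and a repair message to RebootActors.
; Its own Reboot event moves the hub to TPLocation, and Repair clears IsActive so it can be used again.
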(event `self.ReceiveBeginPlay`
  (`parent.ReceiveBeginPlay`)
  (bind _asbp_first_person_character (cast `/Game/FirstPerson/Blueprints/BP_FirstPersonCharacter` (`GameplayStatics.GetPlayerPawn` 0)))
  (set `self.Ded` _asbp_first_person_character))

(event `/Game/Interfaces/BPI_InteractObject.OnInteract`
  (if (not (`self.bIsActive`))
    (`/Game/FirstPerson/Blueprints/BP_FirstPersonCharacter.ReplenishOxygen` (`self.Ded`) 100)
    (`/Game/FirstPerson/Blueprints/BP_FirstPersonCharacter.UpdateUIOxygen` (`self.Ded`))
    (`GameplayStatics.PlaySoundAtLocation` "/Game/Sounds/SW_PickUpOxygenBalloon_variant_1.SW_PickUpOxygenBalloon_variant_1" (`self.K2_GetActorLocation`) (struct) 1.0 1.0 0.0 null null null null)
    (set `self.bIsActive` true)
    (message `/Game/Interfaces/BPI_Reboot.Reboot` (`self.OxygenDoor`))
    (message `/Game/Interfaces/BPI_Reboot.Reboot` (`self.Door`))
    (message `/Game/Interfaces/BPI_Repair.Repair` (`self.RebootActors`) true)))

(event `/Game/Interfaces/BPI_Reboot.Reboot`
  (`self.K2_SetActorLocation` (`self.TPLocation`)))

(event `/Game/Interfaces/BPI_Repair.Repair`
  (params (bIsRepair :type Boolean))
  (set `self.bIsActive` false))

(fn `UserConstructionScript`
  (`parent.UserConstructionScript`))