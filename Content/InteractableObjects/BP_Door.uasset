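; BP_Door is an interactable door that swings open once when OnInteract fires.
; An IsActive flag blocks repeat interactions, and the first one plays the open sound at the door's location and starts a timeline.
; Each timeline update adds the Speed track value to the actor's local yaw, so rotation accumulates per update rather than interpolating to a target angle.
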(event `/Game/Interfaces/BPI_InteractObject.OnInteract`
  (if (not (`self.bIsActive`))
    (`GameplayStatics.PlaySoundAtLocation` "/Game/Sounds/SW_OpenDoor.SW_OpenDoor" (`self.K2_GetActorLocation`) (struct) 1.0 1.0 0.0 null null null null)
    (set `self.bIsActive` true)
    (bind (_direction _speed) (`Timeline|Timeline`)
      (:`Update`
        (`self.K2_AddActorLocalRotation` (`KismetMathLibrary.MakeRotator` 0.0 0.0 _speed))))))

(fn `UserConstructionScript`
  (`parent.UserConstructionScript`))