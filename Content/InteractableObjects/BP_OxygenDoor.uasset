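; BP_OxygenDoor is a door whose timeline slides a Cube vertically, lowered when open and raised when closed.
; Repair clears IsLever and opens the door, while Reboot sets IsLever to suspend the trigger box response.
; With IsLever clear, an actor tagged "1" closes the door on entering the box and reopens it on leaving.
; An IsOpen toggle branch is present but unconnected.
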(event `/Game/Interfaces/BPI_Repair.Repair`
  (params (bIsRepair :type Boolean))
  (set `self.bIsLever` false)
  ; OKAK
  (set `self.bIsOpen` true)
  (bind (_direction _newtrack_0) (`Timeline|TOxygenDoorDown` :!label _label)
    (:`Update`
      (`SceneComponent.K2_SetRelativeLocation` (`self.Cube`) (`KismetMathLibrary.MakeVector` 0.0 0.0 (* _newtrack_0 -100.0)) false false))))

(event `/Game/Interfaces/BPI_Reboot.Reboot`
  (set `self.bIsLever` true))

(event `self.Box.OnComponentBeginOverlap`
  (params (OverlappedComponent :type "PrimitiveComponent Object Reference") (OtherActor :type "Actor Object Reference") (OtherComp :type "PrimitiveComponent Object Reference") (OtherBodyIndex :type Integer) (bFromSweep :type Boolean) (SweepResult :type "HitResult Structure (by ref)"))
  (if (`self.ActorHasTag` OtherActor "1")
    (if (not (`self.bIsLever`))
      (set `self.bIsOpen` false)
      (goto _label :!via `Reverse`))))

(event `self.Box.OnComponentEndOverlap`
  (params (OverlappedComponent :type "PrimitiveComponent Object Reference") (OtherActor :type "Actor Object Reference") (OtherComp :type "PrimitiveComponent Object Reference") (OtherBodyIndex :type Integer))
  (if (`self.ActorHasTag` OtherActor "1")
    (if (not (`self.bIsLever`))
      (set `self.bIsOpen` true)
      (goto _label))))

(fn `UserConstructionScript`)